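; BP_Aldus_NPC is the character Blueprint for the NPC Aldus, who holds conversations with whoever interacts with him.
; On BeginPlay it passes its audio component to BPAldusDialogues and reads his name from the "Aldus" row of StatsTable.
; Interact, skip and close events forward to BPAldusDialogues to open, advance or end the conversation.
; The stored interacting actor receives ConversationClosedMessage when ConversationClosed fires.
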(event EventBeginPlay
  (Default|SetAudioComponentRef (Variables|Default|GetBP_Aldus_Dialogues) (Variables|Default|GetAudio))
  (bind _returnvalue (Utilities|GetDataTableRow (Variables|Default|GetStatsTable) "Aldus")
    (:then
      (Variables|Default|SetName (.Name (Utilities|Struct|BreakS_Player_Stats _returnvalue))))))

(event EventSkipDialogue
  (Default|ProgressDialogue (Variables|Default|GetBP_Aldus_Dialogues)))

(event EventCloseConversation
  (Default|CloseConversation (Variables|Default|GetBP_Aldus_Dialogues)))

(event EventInteract
  (params (InteractActor :type Actor%20Object%20Reference))
  (Variables|Default|SetInteractActor InteractActor)
  (Default|OpenConversation (Variables|Default|GetBP_Aldus_Dialogues)))

(event EventConversationClosed
  (Class|BPIInteractable|ConversationClosed(Message) (Variables|Default|GetInteractActor)))

(fn ConstructionScript
  (|CallParentFunction))