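; Test enemy Blueprint with a health bar widget that appears while the player is locked onto it.
; On spawn it hides the bar and caches the first BP_Player found.
; CheckHealthbarVisibility compares the player's LockOnComponent target to itself, toggling the bar and lock-on sphere.
; While locked, a looping frame-delta timer, rather than Tick, updates the bar from TestStats health and turns it toward the camera.
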(event EventBeginPlay
  ;[0.266 0.266 0.266] Get Da Player reference & Hige HealthBar on Spawn
  (Widget|SetVisibility (UserInterface|GetUserWidgetObject (Variables|Default|GetHealthBarWidget)) "Hidden")
  (CallFunction|GetPlayerRef))

(event EventCheckHealthbarVisibility
  (bind _playerreference (Variables|Default|GetPlayerReference))
  (bind _lockoncomponent (Variables|/Game/ThirdPerson/Blueprints/BP_Player.BP_Player_C|GetLockOnComponent _playerreference))
  (bind _lockonsphere_ref (Variables|/Game/Mecanics/Lock-on/LockOnComponent.LockOnComponent_C|GetLockOnSphere%20Ref _lockoncomponent))
  ;[0.2387 0.2387 0.2387] Check if you hide the HealthBar or not
  (bind _current_target (Default|GetLockonTarget (Variables|/Game/ThirdPerson/Blueprints/BP_Player.BP_Player_C|GetLockOnComponent (Variables|Default|GetPlayerReference))))
  (if (== _current_target self)
    (if (Variables|/Game/Mecanics/Lock-on/LockOnComponent.LockOnComponent_C|GetLockOnAnEnnemy (Variables|/Game/ThirdPerson/Blueprints/BP_Player.BP_Player_C|GetLockOnComponent (Variables|Default|GetPlayerReference)))
      (CallFunction|ShowHealthBar)
      (Default|ShowLockonSphere _lockonsphere_ref)
      (bind _returnvalue (Utilities|Time|SetTimerbyEvent (delegate EventUpdateHealthBarRotation) (Utilities|Time|GetWorldDeltaSeconds) true))
      (else
        (Default|HideLockonSphere _lockonsphere_ref :!label _label)
        (CallFunction|HideHealthBar)
        (CallFunction|StopUpdatingHealthBarRotation)))
    (else
      (goto _label))))

(event EventStopUpdatingHealthBarRotation
  ;[0.2387 0.2387 0.2387] Check if you hide the HealthBar or not
  (Utilities|Time|ClearandInvalidateTimerbyHandle (stale EventCheckHealthbarVisibility _returnvalue)))

(event EventUpdateHealthBarRotation
  (bind _test_stats (Variables|Default|GetTest_Stats))
  (bind _healthbarwidget (Variables|Default|GetHealthBarWidget))
  ;[0.2387 0.2387 0.2387] Check if you hide the HealthBar or not
  (bind _asennemies_health_bar (Utilities|Casting|CastToEnnemiesHealthBar (UserInterface|GetWidget (Variables|Default|GetHealthBarWidget))))
  (Progress|SetPercent (Variables|/Game/Mecanics/Ennemies_HealthBars/EnnemiesHealthBar.EnnemiesHealthBar_C|GetProgressBarofHealthBar _asennemies_health_bar) (* 1e+02 (/ (Variables|/Game/Statistics/Test_Stats.Test_Stats_C|GetHealth _test_stats) (Variables|/Game/Statistics/Test_Stats.Test_Stats_C|GetMaxHealth _test_stats))))
  (Transformation|SetWorldRotation _healthbarwidget (Math|Rotator|FindLookatRotation (Transformation|GetWorldLocation _healthbarwidget) (Transformation|GetWorldLocation (Variables|/Script/Engine.PlayerCameraManager|GetTransformComponent (Game|GetPlayerCameraManager 0)))) false false))

(event EventShowHealthBar
  ;[0.2796 0.2796 0.2796] Show and Hide HealthBar Events
  (Widget|SetVisibility (UserInterface|GetUserWidgetObject (Variables|Default|GetHealthBarWidget)) "Visible"))

(event EventHideHealthBar
  ;[0.2796 0.2796 0.2796] Show and Hide HealthBar Events
  (Widget|SetVisibility (UserInterface|GetUserWidgetObject (Variables|Default|GetHealthBarWidget)) "Hidden"))

(event EventGetPlayerRef
  ;[0.266 0.266 0.266] Get Da Player reference & Hige HealthBar on Spawn
  (bind _outactors (Actor|GetAllActorsOfClass "/Game/ThirdPerson/Blueprints/BP_Player.BP_Player_C"))
  (Variables|Default|SetPlayerReference (Utilities|Array|Get(acopy) _outactors)))

(fn ConstructionScript)