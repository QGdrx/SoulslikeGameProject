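; BP_LockOnComponent is a lock-on component that turns the controller's view toward a Target.
; Its selected, deselected and not-found events only print debug messages, including the selected target's name.
; OnTimer interpolates control pitch and yaw toward a look-at rotation from the player camera to the Target, preserving roll.
; The interpolation uses a hard-coded delta time instead of the real elapsed time.
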(event EventOnTimer
  (params (Controller :type Controller%20Object%20Reference))
  (bind _returnvalue (Game|GetPlayerCameraManager 0))
  (bind _returnvalue_2 (Pawn|GetControlRotation Controller :!class /Script/Engine.Controller))
  (bind _target (Variables|Default|GetTarget))
  (bind _returnvalue_3 (Camera|GetCameraLocation _returnvalue))
  (bind _returnvalue_4 (Transformation|GetWorldLocation _target))
  (bind _returnvalue_5 (Math|Rotator|FindLookatRotation _returnvalue_3 _returnvalue_4))
  (bind _returnvalue_6 (Math|Interpolation|RInterpTo _returnvalue_2 _returnvalue_5 0.2 15.0))
  (Pawn|SetControlRotation Controller (Math|Rotator|MakeRotator (.Roll (Math|Rotator|BreakRotator _returnvalue_2)) (.pitch _returnvalue_6) (.yaw _returnvalue_6))))

(event EventOnTargetDeselected
  (Development|PrintString "Target Deselected" true true "(R=0.000000,G=0.660000,B=1.000000,A=1.000000)" 2.0 "Target"))

(event EventOnTargetSelected
  (params (SelectedTarget :type Sphere%20Component%20Object%20Reference))
  (Development|PrintString (Utilities|String|Append "Target: " (Utilities|GetDisplayName SelectedTarget)) true true "(R=0.000000,G=0.660000,B=1.000000,A=1.000000)" 2.0 "Target"))

(event EventOnTargetNotFound
  (Development|PrintString "No Target Found" true true "(R=0.000000,G=0.660000,B=1.000000,A=1.000000)" 2.0 "Target"))