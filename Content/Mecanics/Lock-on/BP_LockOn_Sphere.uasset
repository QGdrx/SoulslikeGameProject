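; Lock-on indicator actor that shows a sphere slightly above the enemy the player has locked onto.
; It caches the player on BeginPlay and starts hidden; show and hide events check the player's LockOnComponent before toggling visibility.
; When shown, it fetches the lock target and runs a looping timer at the frame delta interval to follow it, clearing that timer when hidden.
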(event Custom|Show%20LockOn%20Sphere
  (if (Variables|/Game/Mecanics/Lock-on/LockOnComponent.LockOnComponent_C|GetLockOnAnEnnemy (Variables|/Game/ThirdPerson/Blueprints/BP_Player.BP_Player_C|GetLockOnComponent (Variables|Default|GetPlayer%20ref)))
    (CallFunction|SetLockonSphereLocation)
    (Rendering|SetVisibility (Variables|Default|GetSphere) true true)
    (Variables|Default|SetVisibility true)))

(event Custom|Hide%20LockOn%20Sphere
  (if (not (Variables|/Game/Mecanics/Lock-on/LockOnComponent.LockOnComponent_C|GetLockOnAnEnnemy (Variables|/Game/ThirdPerson/Blueprints/BP_Player.BP_Player_C|GetLockOnComponent (Variables|Default|GetPlayer%20ref))))
    (CallFunction|StopUpdatingLockonSphereLocation)
    (Rendering|SetVisibility (Variables|Default|GetSphere) false true)
    (Variables|Default|SetVisibility false)))

(event Custom|Set%20LockOnSphere%20Location
  (params (LockOnCollision :type Capsule%20Component%20Object%20Reference))
  (bind _current_target (Default|GetLockonTarget (Variables|/Game/ThirdPerson/Blueprints/BP_Player.BP_Player_C|GetLockOnComponent (Variables|Default|GetPlayer%20ref))))
  (bind _returnvalue (Utilities|Time|SetTimerbyEvent (delegate Custom|Update%20LockOnSphere%20Location) (Utilities|Time|GetWorldDeltaSeconds) true)))

(event Custom|Update%20LockOnSphere%20Location
  (Transformation|SetWorldLocation (Variables|Default|GetSphere) (Math|Vector|MakeVector (.x (Transformation|GetActorLocation (stale Custom|Set%20LockOnSphere%20Location _current_target))) (.y (Transformation|GetActorLocation (stale Custom|Set%20LockOnSphere%20Location _current_target))) (+ (.z (Transformation|GetActorLocation (stale Custom|Set%20LockOnSphere%20Location _current_target))) 4e+01)) false false))

(event Custom|Stop%20Updating%20LockOnSphere%20Location
  (Utilities|Time|ClearandInvalidateTimerbyHandle (stale Custom|Set%20LockOnSphere%20Location _returnvalue)))

(event EventBeginPlay
  (bind _asbp_player (Utilities|Casting|CastToBP_Player (Game|GetPlayerCharacter 0)))
  (Variables|Default|SetPlayer%20ref _asbp_player)
  (Rendering|SetVisibility (Variables|Default|GetSphere) false true))

(fn ConstructionScript)