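; Base NPC Blueprint for the dialogue system that can be interacted with to open a conversation.
; The construction script fills the CharacterName text from SelfName, and SetInteractableState shows or hides that label.
; Interact stores the interacting actor and calls OpenConversation on BPBaseDialogue.
; When the conversation closes, the NPC sends ConversationClosedMessage back to that stored actor.
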(event EventConversationClosed
  (Class|BPIInteractable|ConversationClosed(Message) (Variables|Default|GetInteractActor)))

(event EventInteract
  (params (InteractActor :type Actor%20Object%20Reference))
  (Variables|Default|SetInteractActor InteractActor)
  (Default|OpenConversation (Variables|Default|GetBP_Base_Dialogue)))

(event EventSetInteractableState
  (params (ShowInteract :type Boolean))
  (bind _charactername (Variables|Default|GetCharacterName))
  (if ShowInteract
    (Rendering|SetVisibility _charactername true false)
    (else
      (Rendering|SetVisibility _charactername false false))))

(fn ConstructionScript
  (Rendering|Components|TextRender|SetText (Variables|Default|GetCharacterName) (Variables|Default|GetSelfName)))