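; Base NPC dialogue component that opens a dialogue widget and drives branching conversations with optional audio and montage playback on its owner.
; Each choice is stored by index, then the overridable Dialogue function replays from the start, with AddDialogue passing answered steps and breaking at the first unanswered one.
; Progress can be cleared, rewound or saved via SaveGame.
; Arrays track unlocked and used options, while several option-lookup helpers remain stubs.
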(event Custom|PlayAnimationMontage
  (params (Animation :type Anim%20Montage%20Object%20Reference))
  (Animation|Montage|PlayMontage (Actor|GetComponentbyClass (Components|GetOwner) "/Script/Engine.SkeletalMeshComponent") Animation))

(event Custom|SetAudioComponentRef
  (params (AudioComponent :type Audio%20Component%20Object%20Reference))
  (if (Variables|DialogueSystem|GetUseAudio)
    (Variables|DialogueSystem|SetAudioComponentRef AudioComponent)))

(event EventSaveData
  (params (SaveGameRef :type BP%20Save%20Game%20Object%20Reference))
  (Variables|/Game/Mecanics/SaveSystem/BP_SaveGame.BP_SaveGame_C|SetDialogueProgressAldus SaveGameRef (Variables|DialogueSystem|GetDialogueProgress)))

(event EventLoadData
  (params (SaveGameRef :type BP%20Save%20Game%20Object%20Reference))
  (Variables|DialogueSystem|SetDialogueProgress (Variables|/Game/Mecanics/SaveSystem/BP_SaveGame.BP_SaveGame_C|GetDialogueProgressAldus SaveGameRef)))

(fn OpenConversation
  (bind _returnvalue (UserInterface|CreateWidget "/Game/Mecanics/DialogueSystem/Base/Widgets/WB_Dialogue.WB_Dialogue_C" 0 self))
  (bind _output_get (Variables|DialogueSystem|SetDialogueWidgetRef _returnvalue))
  (UserInterface|Viewport|AddtoViewport _output_get 0)
  (CallFunction|ProgressDialogue))

(fn CloseConversation
  (bind _returnvalue (Components|GetOwner))
  (Widget|RemovefromParent (Variables|DialogueSystem|GetDialogueWidgetRef))
  (bind _audiocomponentref (Variables|DialogueSystem|GetAudioComponentRef)
    (:then
      (Audio|Components|Audio|Stop _audiocomponentref))
    (:else
      _))
  (bind _ascharacter (Utilities|Casting|CastToCharacter _returnvalue)
    (:then
      (Animation|StopAnimMontage _ascharacter 0))
    (:CastFailed
      _))
  (Class|BPIInteractable|ConversationClosed(Message) _returnvalue))

(fn ProgressDialogue
  (Variables|DialogueSystem|SetDialogueIndex -1)
  (CallFunction|Dialogue))

(fn Dialogue)

(fn AddDialogue
  (params (DialogueRow :type S%20Dialogue%20Structure))
  (bind (_npc_name _dialoguetext _responsestext _audio _animation) (Utilities|Struct|BreakS_Dialogue DialogueRow))
  (bind _customoptions (Variables|DialogueSystem|GetCustomOptions))
  (if (Variables|DialogueSystem|GetUseCustomOptions)
    (if (Utilities|Array|IsNotEmpty _customoptions)
      (Variables|DialogueSystem|SetOptionsList _customoptions)
      (else
        (Variables|DialogueSystem|SetOptionsList _responsestext :!label _label)))
    (else
      (goto _label)))
  (bind _result (Math|Integer|IncrementInt (Variables|DialogueSystem|GetDialogueIndex))
    (:%20%20
      (Variables|DialogueSystem|SetDaIndexo _result)
      (if (.ReturnValue (Utilities|Map|Find (Variables|DialogueSystem|GetDialogueProgress) _result))
        (return "NewEnumerator0" (.Value (Utilities|Map|Find (Variables|DialogueSystem|GetDialogueProgress) _result)))
        (else
          (Default|UpdateTextAudioAnimationWB (Variables|DialogueSystem|GetDialogueWidgetRef) _npc_name _dialoguetext _audio _animation (Variables|DialogueSystem|GetOptionsList) (Variables|DialogueSystem|GetDaIndexo) (Variables|OptionSystem|GetUseDynamicOptions))
          (return "NewEnumerator1" 0))))))

(fn UpdateSelectedOption
  (params (DialogueIndex :type Integer) (OptionIndex :type Integer))
  (Variables|/Game/Mecanics/DialogueSystem/Base/Widgets/WB_Dialogue.WB_Dialogue_C|SetOptionsOnScreen (Variables|DialogueSystem|GetDialogueWidgetRef) false)
  (Utilities|Map|Add (Variables|DialogueSystem|GetDialogueProgress) DialogueIndex OptionIndex)
  (CallFunction|ProgressDialogue))

(fn ClearDialogueProgress
  (Utilities|Map|Clear (Variables|DialogueSystem|GetDialogueProgress)))

(fn RemoveDialogueProgress
  (params (ProgressSteps :type Integer))
  (for _index (range 0 ProgressSteps)
    (Utilities|Map|Remove (Variables|DialogueSystem|GetDialogueProgress) (- (Variables|DialogueSystem|GetDialogueIndex) _index))))

(fn SetDialogueBranch
  (params (DialogueBranch :type Name) (ProgressHandler :type E_DialogueState%20Enum :default "NewEnumerator0"))
  (switch Utilities|FlowControl|Switch|SwitchonE_DialogueState ProgressHandler
    (:NewEnumerator0
      (Variables|DialogueSystem|SetActiveDialogueBranch DialogueBranch)
      (CallFunction|ClearDialogueProgress))))

(fn PlayAudio
  (params (Audio :type Sound%20Base%20Object%20Reference%20%28by%20ref%29))
  (bind _audiocomponentref (Variables|DialogueSystem|GetAudioComponentRef))
  (if (Variables|DialogueSystem|GetUseAudio)
    (Utilities|IsValid Audio
      (:Is%20Valid
        (Audio|Components|Audio|SetSound _audiocomponentref Audio)
        (Audio|Components|Audio|Play _audiocomponentref 0.0)
        (return)))))

(fn UpdateUnlockedOptionBools
  (params (OptionsList :type Array%20of%20Integers))
  (for _array_element OptionsList
    (Utilities|Array|SetArrayElem (Variables|OptionSystem|GethasOptionBeenUnlockedByPlayer) _array_element true))
  (Development|PrintString "Updated Unlocked Option Bools")
  (return))

(fn UpdateAlreadyUsedOptionBools
  (params (OptionID :type Integer))
  (Utilities|Array|SetArrayElem (Variables|OptionSystem|GethasOptionAlreadyBeenUsed) OptionID true))

(fn UpdatePlayerOptions
  (bind _playerusableoptions (Variables|OptionSystem|GetPlayerUsableOptions))
  (for (_array_element _array_index) (Variables|OptionSystem|GetAllOptionsList)
    (if (Utilities|Array|Get(acopy) (Variables|OptionSystem|GethasOptionBeenUnlockedByPlayer) _array_index)
      (if (Utilities|Array|Get(acopy) (Variables|OptionSystem|GethasOptionAlreadyBeenUsed) _array_index)
        (Utilities|Array|SetArrayElem _playerusableoptions _array_index "")
        (else
          (Utilities|Array|SetArrayElem _playerusableoptions _array_index _array_element)))))
  (Development|PrintString "Updated Player Options")
  (return))

(fn FindOptionIDinAllOptionList
  (params (CurrentRowID :type Integer) (SelectedOptionID :type Integer))
  (return 0))

(fn MakeSpecialArray
  (params (CurrentRowID :type Integer))
  (return 0))

(fn SetDialogueRow
  (params (CurrentDialogueRow :type Integer) (OptionID :type Integer))
  (return CurrentDialogueRow))

(fn GetDialogueOptionsOfRow
  (params (DataTable :type Data%20Table%20Object%20Reference) (DialogueRow :type Array%20of%20Names) (RowIndex :type Integer))
  (bind _returnvalue (Utilities|GetDataTableRow DataTable (Utilities|Array|Get(acopy) DialogueRow RowIndex))
    (:then
      (return (.ResponsesText (Utilities|Struct|BreakS_Dialogue _returnvalue))))))